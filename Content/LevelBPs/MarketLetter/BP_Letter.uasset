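; BP_Letter is a market letter pickup that advances the player's quest to finding the horn.
; When the ThirdPersonCharacter overlaps its box and PlayerCon has ListenedToPride set, it destroys the letter mesh and trigger and flags ReadLetter.
; OBJCheckpoint then shows the new objective in an Information widget and plays the HUD fade animation.
; It also hides the current objective marker and reveals the next one.
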(event OnComponentBeginOverlap(Box)
  (params (OverlappedComponent :type Primitive%20Component%20Object%20Reference) (OtherActor :type Actor%20Object%20Reference) (OtherComp :type Primitive%20Component%20Object%20Reference) (OtherBodyIndex :type Integer) (bFromSweep :type Boolean) (SweepResult :type Hit%20Result%20Structure%20%28by%20ref%29))
  (Utilities|Casting|CastToThirdPersonCharacter OtherActor)
  (if (Variables|/Game/Mechanics_Blockout/PlayerCon.PlayerCon_C|GetListenedToPride? (.AsPlayer%20Con (Utilities|Casting|CastToPlayerCon (Game|GetPlayerController 0))))
    (Components|DestroyComponent (Variables|Default|GetLetterMesh))
    (CallFunction|OBJCheckpoint "The horn" "Find the horn in the big building East of the market ")
    (Variables|/Game/Mechanics_Blockout/PlayerCon.PlayerCon_C|SetReadLetter? (.AsPlayer%20Con (Utilities|Casting|CastToPlayerCon (Game|GetPlayerController 0))) true)
    (Rendering|SetVisibility (Variables|/Game/LevelBPs/TempObjMarker/BP_TempOBJMarker4.BP_TempOBJMarker4_C|GetMarker%20Widget (Variables|Default|GetObjMarkerBP)) false false)
    (Rendering|SetVisibility (Variables|/Game/LevelBPs/TempObjMarker/BP_TempOBJMarker5.BP_TempOBJMarker5_C|GetMarker%20Widget (Variables|Default|GetObjMarkerBP2)) true false)
    (Components|DestroyComponent (Variables|Default|GetBox))))

(fn ConstructionScript)

(fn OBJCheckpoint
  (params (Title :type Text) (Desc :type Text))
  (bind _returnvalue (Game|GetPlayerCharacter 0))
  (bind _asthird_person_character (Utilities|Casting|CastToThirdPersonCharacter _returnvalue))
  (bind _hud (Variables|/Game/ThirdPersonBP/Blueprints/ThirdPersonCharacter.ThirdPersonCharacter_C|GetHUD _asthird_person_character))
  (bind _returnvalue_2 (UserInterface|CreateWidget "/Game/UI/Widget/Information.Information_C"))
  (Default|UpdateHud _returnvalue_2 Title Desc (Variables|Default|GetIcon))
  (UserInterface|Viewport|AddtoViewport _returnvalue_2 0)
  (UserInterface|Animation|PlayAnimation _hud (Variables|/Game/UI/Widget/HUD.HUD_C|GetFade _hud) 0.0 1 "Forward" 1.0 false))