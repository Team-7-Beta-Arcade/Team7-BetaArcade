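; BP_PrideDialogue is a trigger actor that plays a short scripted Pride spirit dialogue and then gives the player a new objective.
; A box overlap disables input on the overlapping actor, shows two lines in timed sequence, then re-enables input on the player character.
; OBJCheckpoint then displays an Information widget pointing to a letter about the horn's location, and the box destroys itself so the dialogue plays once.
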(event OnComponentBeginOverlap(Box)
  (params (OverlappedComponent :type Primitive%20Component%20Object%20Reference) (OtherActor :type Actor%20Object%20Reference) (OtherComp :type Primitive%20Component%20Object%20Reference) (OtherBodyIndex :type Integer) (bFromSweep :type Boolean) (SweepResult :type Hit%20Result%20Structure%20%28by%20ref%29))
  (Input|DisableInput OtherActor (Game|GetPlayerController 0))
  (Rendering|SetVisibility (Variables|Default|GetLine_01) true false)
  (Utilities|FlowControl|Delay 2.0)
  (Rendering|SetVisibility (Variables|Default|GetLine_01) false false)
  (Rendering|SetVisibility (Variables|Default|GetLine_02) true false)
  (Utilities|FlowControl|Delay 2.0)
  (Rendering|SetVisibility (Variables|Default|GetLine_02) false false)
  (Input|EnableInput (Game|GetPlayerCharacter 0) (Game|GetPlayerController 0))
  (CallFunction|OBJCheckpoint "Letter" "Find letter showing location of the horn")
  (Components|DestroyComponent (Variables|Default|GetBox)))

(fn ConstructionScript)

(fn OBJCheckpoint
  (params (Title :type Text) (Desc :type Text))
  (bind _returnvalue (UserInterface|CreateWidget "/Game/UI/Widget/Information.Information_C"))
  (Default|Update _returnvalue Title Desc (Variables|Default|GetIcon))
  (UserInterface|Viewport|AddtoViewport _returnvalue 0))