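; Blockout destructible wall that breaks when an Enemy of one specific EmotionType charges into it.
; The Destructible component's hit event checks that type and charge state, then enables physics and applies damage plus an impulse along the hit normal.
; It then ignores the Pawn channel and plays a 2D hit sound.
; A throwable-item trigger and a delay are left unconnected.
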(event OnComponentHit(Destructible)
  (params (HitComponent :type Primitive%20Component%20Object%20Reference) (OtherActor :type Actor%20Object%20Reference) (OtherComp :type Primitive%20Component%20Object%20Reference) (NormalImpulse :type Vector :default "0, 0, 0") (Hit :type Hit%20Result%20Structure%20%28by%20ref%29))
  (bind _asenemy (Utilities|Casting|CastToEnemy OtherActor))
  (if (Utilities|Enum|Equal(Enum) (Variables|/Game/Mechanics_Blockout/AI/Enemy.Enemy_C|GetEmotionType _asenemy) "NewEnumerator0")
    (if (Variables|/Game/Mechanics_Blockout/AI/Enemy.Enemy_C|GetIsCharging? _asenemy)
      (bind _output_get (Variables|Default|SetHit%20Location (.location Hit)))
      (bind _output_get_2 (Variables|Default|SetNormal%20Impulse (* NormalImpulse 1)))
      (Physics|SetSimulatePhysics (Variables|Default|GetDestructible) true)
      (Class|DestructibleComponent|ApplyDamage (Variables|Default|GetDestructible) 1e+01 _output_get _output_get_2 1e+04)
      (Physics|AddImpulse (Variables|Default|GetDestructible) (* (Math|Vector|Normalize _output_get_2) 4e+02) "None" true)
      (Collision|SetCollisionResponsetoChannel (Variables|Default|GetDestructible) "ECC_Pawn" "ECR_Ignore")
      (Audio|PlaySound2D "/Game/SFX/DestructibleHit_Cue.DestructibleHit_Cue" 1.0 1.0 0.0 0 0))))

(event EventBeginPlay)

(event Collision|EventActorBeginOverlap
  (params (OtherActor :type Actor%20Object%20Reference)))

(event EventTick
  (params (DeltaSeconds :type Float%20%28single-precision%29)))

(fn ConstructionScript)