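; Letter_BP is a blockout readable letter that switches the player's view to itself when the ThirdPersonCharacter overlaps its box.
; On overlap it blends the camera to the letter and disables player input for a few seconds.
; A looping timer meanwhile polls whether the character is moving, then blends the view back to the player and pauses itself.
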(event OnComponentBeginOverlap(Box)
  (params (OverlappedComponent :type Primitive%20Component%20Object%20Reference) (OtherActor :type Actor%20Object%20Reference) (OtherComp :type Primitive%20Component%20Object%20Reference) (OtherBodyIndex :type Integer) (bFromSweep :type Boolean) (SweepResult :type Hit%20Result%20Structure%20%28by%20ref%29))
  (bind _returnvalue (Game|GetPlayerController 0))
  (bind _returnvalue_2 (Game|GetPlayerCharacter 0))
  (Utilities|Casting|CastToThirdPersonCharacter OtherActor)
  ;[1 1 1] start reading
  (Game|Player|SetViewTargetwithBlend (Game|GetPlayerController 0) self 2.0 "VTBlend_EaseInOut" 4.0 false)
  (Utilities|FlowControl|Sequence
    (:then_0
      ;[1 1 1] Input disable/Enable
      (Input|DisableInput _returnvalue_2 _returnvalue)
      (Utilities|FlowControl|Delay 4.0)
      (Input|EnableInput _returnvalue_2 _returnvalue))
    (:then_1
      ;[1 1 1] Stop reading
      (bind _returnvalue_3 (Utilities|Time|SetTimerbyEvent (delegate Custom|Stop%20reading) 0.05 true 4.0)))))

(event Custom|Stop%20reading
  ;[1 1 1] Stop reading
  (if (Default|IsMoving? (.AsThird%20Person%20Character (Utilities|Casting|CastToThirdPersonCharacter (Game|GetPlayerCharacter 0))))
    (Game|Player|SetViewTargetwithBlend (Game|GetPlayerController 0) (Game|GetPlayerCharacter 0) 2.0 "VTBlend_EaseInOut" 4.0 false)
    (Utilities|Time|PauseTimerbyHandle (stale OnComponentBeginOverlap(Box) _returnvalue_3))))

(event EventBeginPlay)

(fn ConstructionScript)