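; BP_Shadow is a moving shadow zone that tells the player character when it is inside shadow.
; A looping latent MoveComponentTo eases the root toward the Box's location, while a delayed Return event sends it back.
; Sphere overlaps set the character's InShadow flag and call BlendWithShadows with this actor.
; Exit overlaps are ignored while the player controller is teleporting.
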(event OnComponentBeginOverlap(Sphere)
  (params (OverlappedComponent :type Primitive%20Component%20Object%20Reference) (OtherActor :type Actor%20Object%20Reference) (OtherComp :type Primitive%20Component%20Object%20Reference) (OtherBodyIndex :type Integer) (bFromSweep :type Boolean) (SweepResult :type Hit%20Result%20Structure%20%28by%20ref%29))
  (bind _returnvalue (Game|GetPlayerCharacter 0))
  (bind _asthird_person_character (Utilities|Casting|CastToThirdPersonCharacter _returnvalue))
  (if (== OtherActor _returnvalue)
    (Development|PrintString "ShadowTriggered: ENTER" true true "(R=0.090252,G=0.000000,B=1.000000,A=1.000000)" 4.0)
    (Variables|/Game/ThirdPersonBP/Blueprints/ThirdPersonCharacter.ThirdPersonCharacter_C|SetInShadow? _asthird_person_character true)
    (Default|BlendwithShadows _asthird_person_character self)))

(event OnComponentEndOverlap(Sphere)
  (params (OverlappedComponent :type Primitive%20Component%20Object%20Reference) (OtherActor :type Actor%20Object%20Reference) (OtherComp :type Primitive%20Component%20Object%20Reference) (OtherBodyIndex :type Integer))
  (bind _returnvalue (Game|GetPlayerCharacter 0))
  (bind _asthird_person_character (Utilities|Casting|CastToThirdPersonCharacter _returnvalue))
  (if (== OtherActor _returnvalue)
    (if (not (Variables|/Game/Mechanics_Blockout/BP_PlayerCon.BP_PlayerCon_C|GetIsTeleporting? (.AsBP%20Player%20Con (Utilities|Casting|CastToBP_PlayerCon (Game|GetPlayerController 0)))))
      (Development|PrintString "ShadowTriggered: EXIT" true true "(R=0.090252,G=0.000000,B=1.000000,A=1.000000)" 4.0)
      (Variables|/Game/ThirdPersonBP/Blueprints/ThirdPersonCharacter.ThirdPersonCharacter_C|SetInShadow? _asthird_person_character false)
      (Default|BlendwithShadows _asthird_person_character self))))

(event Custom|Return
  (Utilities|FlowControl|Delay 6.0)
  (Components|MoveComponentTo (Variables|Default|GetDefaultSceneRoot) (Transformation|GetWorldLocation (Variables|Default|GetBox)) "0, 0, 0" true true 6.5 false) ; enters at Return
)

(event EventBeginPlay
  (CallFunction|Return :!label _label)
  (Components|MoveComponentTo (Variables|Default|GetDefaultSceneRoot) (Transformation|GetWorldLocation (Variables|Default|GetBox)) "0, 0, 0" true true 6.5 false)
  (Utilities|FlowControl|Delay 2.0)
  (goto _label))

(fn ConstructionScript)