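; Player controller for a third-person character that possesses enemies and teleports between shadow targets.
; V releases any possessed enemy to its AI controller, or requires the player be unseen, then teleports to the TeleportComponenet's target.
; A timeline lerps location, camera FOV, particle and mesh visibility, with play rate scaled by distance.
; PossessionTimer ejects the player after a fixed delay, restoring collision and visibility.
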(event Custom|PossessionTimer
  (bind _returnvalue (Pawn|GetControlledPawn))
  ;[1 1 1] Possession timer
  (Utilities|FlowControl|Delay 4.0) ; Time Player can stay in possession
  (Utilities|Casting|CastToThirdPersonCharacter _returnvalue
    (:CastFailed
      (Default|ChangeEmotion (.AsEnemy (Utilities|Casting|CastToEnemy _returnvalue)) "NewEnumerator0")
      (CallFunction|KickPlayerOutOffPossession)
      (Default|BWSRevealPlayer (Variables|Default|GetPlayerPawn_REF)))))

(event EventPossess
  (params (PossessedPawn :type Pawn%20Object%20Reference))
  ;[1 1 1] DoWhenPossessing a new pawn
  (Default|CheckOwner (Variables|Default|GetTeleportComponenet))
  (if (not (== PossessedPawn "/Game/ThirdPersonBP/Blueprints/ThirdPersonCharacter.ThirdPersonCharacter"))
    (Utilities|FlowControl|Gate true
      (:Exit
        (Default|LookforTP (Variables|Default|GetTeleportComponenet))))))

(event EventBeginPlay
  ;[1 1 1] Beginplay
  (Variables|Default|SetPlayerPawn_REF (.AsThird%20Person%20Character (Utilities|Casting|CastToThirdPersonCharacter (Pawn|GetControlledPawn))))
  (Utilities|FlowControl|Delay 0.5)
  ;[1 1 1] DoWhenPossessing a new pawn
  (Utilities|FlowControl|Gate true) ; enters at Open
)

(event Input|KeyboardEvents|V
  (params (Key :type Key%20Structure))
  (bind _playerpawn_ref (Variables|Default|GetPlayerPawn_REF))
  (bind _playerpawn_ref_2 (Variables|Default|GetPlayerPawn_REF))
  (bind _teleportparticle (Variables|/Game/ThirdPersonBP/Blueprints/ThirdPersonCharacter.ThirdPersonCharacter_C|GetTeleportParticle _playerpawn_ref))
  (bind _returnvalue (Transformation|GetWorldTransform _teleportparticle))
  (:Pressed
    (if (Variables|/Game/ThirdPersonBP/Blueprints/ThirdPersonCharacter.ThirdPersonCharacter_C|GetIsPossessing? (Variables|Default|GetPlayerPawn_REF))
      (Pawn|Possess (Variables|/Game/ThirdPersonBP/Blueprints/ThirdPersonCharacter.ThirdPersonCharacter_C|GetCurrentPossessedAI_Controler (Variables|Default|GetPlayerPawn_REF)) (Pawn|GetControlledPawn))
      (Pawn|Possess (Game|GetPlayerController 0) (Variables|Default|GetPlayerPawn_REF))
      (Variables|/Game/ThirdPersonBP/Blueprints/ThirdPersonCharacter.ThirdPersonCharacter_C|SetIsPossessing? (Variables|Default|GetPlayerPawn_REF) false)
      (Transformation|DetachFromActor _playerpawn_ref_2 "KeepWorld" "KeepWorld" "KeepWorld")
      (Collision|SetCollisionEnabled (Variables|/Script/Engine.Character|GetCapsuleComponent _playerpawn_ref_2) "QueryAndPhysics")
      (Collision|SetCollisionEnabled (Variables|/Script/Engine.Character|GetMesh _playerpawn_ref_2) "QueryAndPhysics")
      (Default|ChangeEmotion (.AsEnemy (Utilities|Casting|CastToEnemy (Pawn|GetControlledPawn))) "NewEnumerator0")
      (Variables|/Game/Mechanics_Blockout/BP_TeleportComponenet.BP_TeleportComponenet_C|GetCurrentTarget (Variables|Default|GetTeleportComponenet) :!label _label
        (:then
          (Default|BlendPossesion (Variables|Default|GetPlayerPawn_REF))
          (Audio|SpawnSoundAttached "/Game/SFX/ShadowTPSound_Cue.ShadowTPSound_Cue" (Variables|/Script/Engine.Character|GetMesh (Variables|Default|GetPlayerPawn_REF)) "None" "0, 0, 0" "0, 0, 0" "KeepRelativeOffset" false 1.0 1.0 0.0 0 0)
          (Variables|Default|SetIsTeleporting? true)
          (Components|Timeline|SetPlayRate (Variables|Default|GetTimeline_Teleport) (/ 1.0 (/ (Math|Vector|Distance(Vector) (Transformation|GetActorLocation (Variables|Default|GetPlayerPawn_REF)) (Transformation|GetWorldLocation (Variables|/Game/Mechanics_Blockout/ActorShadowTest.ActorShadowTest_C|GetCube (Variables|/Game/Mechanics_Blockout/BP_TeleportComponenet.BP_TeleportComponenet_C|GetCurrentTarget (Variables|Default|GetTeleportComponenet))))) 1e+03)))
          (Development|PrintString (Utilities|String|ToString(Float) (Math|Vector|Distance(Vector) (Transformation|GetActorLocation (Variables|Default|GetPlayerPawn_REF)) (Transformation|GetWorldLocation (Variables|/Game/Mechanics_Blockout/ActorShadowTest.ActorShadowTest_C|GetCube (Variables|/Game/Mechanics_Blockout/BP_TeleportComponenet.BP_TeleportComponenet_C|GetCurrentTarget (Variables|Default|GetTeleportComponenet)))))))
          (bind _returnvalue_2 (Effects|SpawnEmitteratLocation "/Game/VFX/InfinityBladeEffects/Particles/P_Skill_Telecharge_Ice_Proj_02.P_Skill_Telecharge_Ice_Proj_02" (.location _returnvalue) (.rotation _returnvalue)))
          (Variables|Default|SetPlayerRotation (CallFunction|FindRotation))
          (bind _tp_track (Timeline|Timeline_Teleport PlayFromStart)
            (:Update
              (Transformation|SetActorLocation (Variables|Default|GetPlayerPawn_REF) (Math|Vector|Lerp(Vector) (Transformation|GetActorLocation (Variables|Default|GetPlayerPawn_REF)) (+ (Transformation|GetWorldLocation (Variables|/Game/Mechanics_Blockout/ActorShadowTest.ActorShadowTest_C|GetCube (Variables|/Game/Mechanics_Blockout/BP_TeleportComponenet.BP_TeleportComponenet_C|GetCurrentTarget (Variables|Default|GetTeleportComponenet)))) "0, 0,96.000000") _tp_track) false false)
              (Camera|SetFieldOfView (Variables|/Game/ThirdPersonBP/Blueprints/ThirdPersonCharacter.ThirdPersonCharacter_C|GetFollowCamera (Variables|Default|GetPlayerPawn_REF)) (Math|Float|Lerp 1.1e+02 9e+01 _tp_track))
              (Transformation|SetWorldLocationAndRotation _returnvalue_2 (Math|Vector|Lerp(Vector) (Transformation|GetActorLocation (Variables|Default|GetPlayerPawn_REF)) (+ (Transformation|GetWorldLocation (Variables|/Game/Mechanics_Blockout/ActorShadowTest.ActorShadowTest_C|GetCube (Variables|/Game/Mechanics_Blockout/BP_TeleportComponenet.BP_TeleportComponenet_C|GetCurrentTarget (Variables|Default|GetTeleportComponenet)))) "0, 0,96.000000") _tp_track) (Variables|Default|GetPlayerRotation) false false)
              (Rendering|SetVisibility (Variables|/Script/Engine.Character|GetMesh (Variables|Default|GetPlayerPawn_REF)) (>= (Math|Float|Lerp 0.0 1.0 _tp_track) 0.6) false))
            (:Finished
              (Default|BWSRevealPlayer (Variables|Default|GetPlayerPawn_REF))
              (Variables|Default|SetIsTeleporting? false)
              (Default|LookforTP (Variables|Default|GetTeleportComponenet))
              (Variables|/Game/Mechanics_Blockout/BP_TeleportComponenet.BP_TeleportComponenet_C|SetCurrentTarget (Variables|Default|GetTeleportComponenet) 0))))
        (:else
          (Rendering|SetVisibility (Variables|/Script/Engine.Character|GetMesh (Variables|Default|GetPlayerPawn_REF)) true false)
          (Default|BWSRevealPlayer (Variables|Default|GetPlayerPawn_REF))))
      (elif (not (Variables|/Game/ThirdPersonBP/Blueprints/ThirdPersonCharacter.ThirdPersonCharacter_C|GetCanBeSeen? (Variables|Default|GetPlayerPawn_REF)))
        (if (not (== (Variables|Default|GetCurrentOccupiedShadow) (Variables|/Game/Mechanics_Blockout/BP_TeleportComponenet.BP_TeleportComponenet_C|GetCurrentTarget (Variables|Default|GetTeleportComponenet))))
          (goto _label))))))

(fn ConstructionScript)

(fn KickPlayerOutOffPossession
  (bind _playerpawn_ref (Variables|Default|GetPlayerPawn_REF))
  (bind _playerpawn_ref_2 (Variables|Default|GetPlayerPawn_REF))
  (bind _capsulecomponent (Variables|/Script/Engine.Character|GetCapsuleComponent _playerpawn_ref_2))
  (Pawn|Possess (Variables|/Game/ThirdPersonBP/Blueprints/ThirdPersonCharacter.ThirdPersonCharacter_C|GetCurrentPossessedAI_Controler (Variables|Default|GetPlayerPawn_REF)) (Pawn|GetControlledPawn))
  (Pawn|Possess (Game|GetPlayerController 0) (Variables|Default|GetPlayerPawn_REF))
  (Variables|/Game/ThirdPersonBP/Blueprints/ThirdPersonCharacter.ThirdPersonCharacter_C|SetIsPossessing? (Variables|Default|GetPlayerPawn_REF) false)
  (Transformation|SetWorldLocation _capsulecomponent (+ (* (* (Math|Vector|GetForwardVector _capsulecomponent) -1.0) 5.0) (Transformation|GetActorLocation _playerpawn_ref_2)) false false)
  (Transformation|DetachFromActor _playerpawn_ref "KeepWorld" "KeepWorld" "KeepWorld")
  (Collision|SetCollisionEnabled (Variables|/Script/Engine.Character|GetCapsuleComponent _playerpawn_ref) "QueryAndPhysics")
  (Collision|SetCollisionEnabled (Variables|/Script/Engine.Character|GetMesh _playerpawn_ref) "QueryAndPhysics")
  (Rendering|SetVisibility (Variables|/Script/Engine.Character|GetMesh (Variables|Default|GetPlayerPawn_REF)) true false))

(fn FindRotation
  (return (Math|Rotator|FindLookatRotation (Transformation|GetActorLocation (Variables|Default|GetPlayerPawn_REF)) (Transformation|GetWorldLocation (Variables|/Game/Mechanics_Blockout/ActorShadowTest.ActorShadowTest_C|GetCube (Variables|/Game/Mechanics_Blockout/BP_TeleportComponenet.BP_TeleportComponenet_C|GetCurrentTarget (Variables|Default|GetTeleportComponenet)))))))