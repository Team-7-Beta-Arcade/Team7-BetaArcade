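; BP_EmotionWell is a pickup that gives the player the emotion set by its EmotionType.
; Its construction script picks the orb material and particle template from that type, with particles only for Anger and Sad.
; It plays an attached sound and bobs on a looping MoveComponentTo.
; On player overlap it sets the character's held emotion, updates the HUD, shows an Information popup and destroys itself.
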(event OnComponentBeginOverlap(Sphere1)
  (params (OverlappedComponent :type Primitive%20Component%20Object%20Reference) (OtherActor :type Actor%20Object%20Reference) (OtherComp :type Primitive%20Component%20Object%20Reference) (OtherBodyIndex :type Integer) (bFromSweep :type Boolean) (SweepResult :type Hit%20Result%20Structure%20%28by%20ref%29))
  (bind _returnvalue (Game|GetPlayerCharacter 0))
  (bind _emotiontype (Variables|Default|GetEmotionType))
  (bind _asthird_person_character (Utilities|Casting|CastToThirdPersonCharacter _returnvalue))
  (bind _hud (Variables|/Game/ThirdPersonBP/Blueprints/ThirdPersonCharacter.ThirdPersonCharacter_C|GetHUD _asthird_person_character))
  (if (== OtherActor _returnvalue)
    (Default|SetCurrentHeldEmotion _asthird_person_character _emotiontype)
    (Default|Update _hud)
    (bind _returnvalue_2 (UserInterface|CreateWidget "/Game/UI/Widget/Information.Information_C"))
    (Default|Update _returnvalue_2 (.Value (Utilities|Map|Find (Variables|Default|GetDictionary) _emotiontype)) "Emotion" (.Value (Utilities|Map|Find (Variables|/Game/UI/Widget/HUD.HUD_C|GetEmotions _hud) _emotiontype)))
    (UserInterface|Viewport|AddtoViewport _returnvalue_2 0)
    (Actor|DestroyActor)))

(event Custom|Return
  (bind _defaultsceneroot (Variables|Default|GetDefaultSceneRoot))
  ;[1 1 1] Basic Anim/ Useless
  (Utilities|FlowControl|Delay 1.5)
  (Components|MoveComponentTo _defaultsceneroot (+ (Transformation|GetWorldLocation _defaultsceneroot) "0, 0,50.000000") (Transformation|GetWorldRotation _defaultsceneroot) true true 1.6 false) ; enters at Return
)

(event EventBeginPlay
  (bind _defaultsceneroot (Variables|Default|GetDefaultSceneRoot))
  (Audio|SpawnSoundAttached "/Game/SFX/EmotionWell_Cue.EmotionWell_Cue" (Variables|Default|GetDefaultSceneRoot) "None" "0, 0, 0" "0, 0, 0" "KeepRelativeOffset" false 1.0 1.0 0.0 0 0)
  ;[1 1 1] Basic Anim/ Useless
  (CallFunction|Return :!label _label)
  (Components|MoveComponentTo _defaultsceneroot (+ (Transformation|GetWorldLocation _defaultsceneroot) "0, 0,50.000000") (Transformation|GetWorldRotation _defaultsceneroot) true true 1.6 false)
  (goto _label))

(fn ConstructionScript
  (Effects|Components|ParticleSystem|SetTemplate (Variables|Default|GetParticleSystem) (Utilities|Select :Index (Variables|Default|GetEmotionType) :NewEnumerator3 0 :NewEnumerator0 "/Game/VFX/InfinityBladeEffects/Particles/P_Summon_Parent_01.P_Summon_Parent_01" :NewEnumerator1 "/Game/VFX/InfinityBladeEffects/Particles/P_Summon_Parent_02.P_Summon_Parent_02" :NewEnumerator2 0 :NewEnumerator4 0 :NewEnumerator5 0))
  (Rendering|Material|SetMaterial (Variables|Default|GetSphere) 0 (Utilities|Select :Index (Variables|Default|GetEmotionType) :NewEnumerator3 "/Game/Mechanics_Blockout/Materials/M_Mechanics_Basic_Black_Inst.M_Mechanics_Basic_Black_Inst" :NewEnumerator0 "/Game/Materials/M_Angryorb.M_Angryorb" :NewEnumerator1 "/Game/Materials/M_Saddnessorb.M_Saddnessorb" :NewEnumerator2 "/Game/Mechanics_Blockout/Materials/M_Mechanics_Basic_Green_Inst.M_Mechanics_Basic_Green_Inst" :NewEnumerator4 "/Game/Mechanics_Blockout/Materials/M_Mechanics_Basic_Yellow_Inst.M_Mechanics_Basic_Yellow_Inst" :NewEnumerator5 "/Game/Mechanics_Blockout/Materials/M_Mechanics_Basic_Grey_Inst.M_Mechanics_Basic_Grey_Inst")))