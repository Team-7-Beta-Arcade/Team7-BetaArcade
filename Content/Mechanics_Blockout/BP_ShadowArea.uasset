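; BP_ShadowArea is a placeable shadow volume that tracks when the player character stands in shadow.
; Its construction script adds a box, sphere or capsule from CollisionType, ignoring one custom trace channel, with collision toggled by StartActive.
; Entering sets InShadow, calls BlendWithShadows, records the shadow point on the player controller and deactivates it.
; Leaving clears the state unless the player is teleporting, without reactivating the point.
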(event OnComponentBeginOverlap(CapsuleComponent)
  (params (OverlappedComponent :type Primitive%20Component%20Object%20Reference) (OtherActor :type Actor%20Object%20Reference) (OtherComp :type Primitive%20Component%20Object%20Reference) (OtherBodyIndex :type Integer) (bFromSweep :type Boolean) (SweepResult :type Hit%20Result%20Structure%20%28by%20ref%29))
  (CallFunction|EnterShadow OtherActor))

(event OnComponentEndOverlap(CapsuleComponent)
  (params (OverlappedComponent :type Primitive%20Component%20Object%20Reference) (OtherActor :type Actor%20Object%20Reference) (OtherComp :type Primitive%20Component%20Object%20Reference) (OtherBodyIndex :type Integer))
  (CallFunction|LeaveShadow OtherActor))

(event OnComponentBeginOverlap(SphereComponent)
  (params (OverlappedComponent :type Primitive%20Component%20Object%20Reference) (OtherActor :type Actor%20Object%20Reference) (OtherComp :type Primitive%20Component%20Object%20Reference) (OtherBodyIndex :type Integer) (bFromSweep :type Boolean) (SweepResult :type Hit%20Result%20Structure%20%28by%20ref%29))
  (CallFunction|EnterShadow OtherActor))

(event OnComponentEndOverlap(SphereComponent)
  (params (OverlappedComponent :type Primitive%20Component%20Object%20Reference) (OtherActor :type Actor%20Object%20Reference) (OtherComp :type Primitive%20Component%20Object%20Reference) (OtherBodyIndex :type Integer))
  (CallFunction|LeaveShadow OtherActor))

(event OnComponentBeginOverlap(BoxComponent)
  (params (OverlappedComponent :type Primitive%20Component%20Object%20Reference) (OtherActor :type Actor%20Object%20Reference) (OtherComp :type Primitive%20Component%20Object%20Reference) (OtherBodyIndex :type Integer) (bFromSweep :type Boolean) (SweepResult :type Hit%20Result%20Structure%20%28by%20ref%29))
  (CallFunction|EnterShadow OtherActor))

(event OnComponentEndOverlap(BoxComponent)
  (params (OverlappedComponent :type Primitive%20Component%20Object%20Reference) (OtherActor :type Actor%20Object%20Reference) (OtherComp :type Primitive%20Component%20Object%20Reference) (OtherBodyIndex :type Integer))
  (CallFunction|LeaveShadow OtherActor))

(event EventBeginPlay)

(fn ConstructionScript
  (switch Utilities|FlowControl|Switch|SwitchonCollisionType_ShadowArea (Variables|Default|GetCollisionType)
    (:NewEnumerator0
      (bind _returnvalue (AddComponent|AddBoxComponent false))
      (Variables|Default|SetBoxComponent _returnvalue)
      (Components|Box|SetBoxExtent _returnvalue (Variables|Default|GetBox%20Extend) true)
      (Collision|SetCollisionResponsetoChannel _returnvalue "ECC_GameTraceChannel1" "ECR_Ignore"))
    (:NewEnumerator1
      (bind _returnvalue_2 (AddComponent|AddSphereComponent false))
      (Variables|Default|SetSphereComponent _returnvalue_2)
      (Components|Sphere|SetSphereRadius _returnvalue_2 (Variables|Default|GetSphere%20Radius) true)
      (Collision|SetCollisionResponsetoChannel _returnvalue_2 "ECC_GameTraceChannel1" "ECR_Ignore"))
    (:NewEnumerator2
      (bind _returnvalue_3 (AddComponent|AddCapsuleComponent false))
      (Variables|Default|SetCapsuleComponent _returnvalue_3)
      (Components|Capsule|SetCapsuleSize _returnvalue_3 (Variables|Default|GetCapsuleSize) (Variables|Default|GetCapsule%20Half%20Height') true)
      (Collision|SetCollisionResponsetoChannel _returnvalue_3 "ECC_GameTraceChannel1" "ECR_Ignore")))
  (Collision|SetActorEnableCollision (Variables|Default|GetStartActive?)))

(fn EnterShadow
  (params (ActorOverlap :type Object%20Object%20Reference))
  (bind _returnvalue (Game|GetPlayerCharacter 0))
  (bind _bp_shadowcomponenet (Variables|Default|GetBP_ShadowComponenet))
  (bind _asthird_person_character (Utilities|Casting|CastToThirdPersonCharacter _returnvalue))
  (bind _shadowpoint (Variables|/Game/Mechanics_Blockout/BP_ShadowComponenet.BP_ShadowComponenet_C|GetShadowPoint _bp_shadowcomponenet))
  (if (== ActorOverlap _returnvalue)
    (Development|PrintString "ShadowTriggered: ENTER" true true "(R=0.090252,G=0.000000,B=1.000000,A=1.000000)" 4.0)
    (Variables|/Game/ThirdPersonBP/Blueprints/ThirdPersonCharacter.ThirdPersonCharacter_C|SetInShadow? _asthird_person_character true)
    (Default|BlendwithShadows _asthird_person_character self)
    (Variables|/Game/Mechanics_Blockout/BP_PlayerCon.BP_PlayerCon_C|SetCurrentOccupiedShadow (.AsBP%20Player%20Con (Utilities|Casting|CastToBP_PlayerCon (Game|GetPlayerController 0))) _shadowpoint)
    (Default|SetActive _shadowpoint false)))

(fn LeaveShadow
  (params (ActorOverlap :type Object%20Object%20Reference))
  (bind _returnvalue (Game|GetPlayerCharacter 0))
  (bind _asthird_person_character (Utilities|Casting|CastToThirdPersonCharacter _returnvalue))
  (if (== ActorOverlap _returnvalue)
    (if (not (Variables|/Game/Mechanics_Blockout/BP_PlayerCon.BP_PlayerCon_C|GetIsTeleporting? (.AsBP%20Player%20Con (Utilities|Casting|CastToBP_PlayerCon (Game|GetPlayerController 0)))))
      (Development|PrintString "ShadowTriggered: EXIT" true true "(R=0.090252,G=0.000000,B=1.000000,A=1.000000)" 4.0)
      (Variables|/Game/ThirdPersonBP/Blueprints/ThirdPersonCharacter.ThirdPersonCharacter_C|SetInShadow? _asthird_person_character false)
      (Default|BlendwithShadows _asthird_person_character self)
      (Variables|/Game/Mechanics_Blockout/BP_PlayerCon.BP_PlayerCon_C|SetCurrentOccupiedShadow (.AsBP%20Player%20Con (Utilities|Casting|CastToBP_PlayerCon (Game|GetPlayerController 0))) 0))))