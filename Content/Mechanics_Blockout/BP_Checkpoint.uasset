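; BP_Checkpoint is a one-shot checkpoint trigger that saves its own location as the player's checkpoint.
; When an actor instigated by a PlayerCon controller overlaps its Box, it loads the existing "CheckpointSave" slot, writes its root location into checpointSaveinfo.PlayerLoc and saves it back.
; It then prints the location and destroys itself.
; An unconnected leftover would have set LastCheckpointLocation on ThirdPersonCharacter.
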(event OnComponentBeginOverlap(Box)
  (params (OverlappedComponent :type Primitive%20Component%20Object%20Reference) (OtherActor :type Actor%20Object%20Reference) (OtherComp :type Primitive%20Component%20Object%20Reference) (OtherBodyIndex :type Integer) (bFromSweep :type Boolean) (SweepResult :type Hit%20Result%20Structure%20%28by%20ref%29))
  (Utilities|Casting|CastToPlayerCon (Game|GetInstigatorController OtherActor))
  (bind _returnvalue (SaveGame|LoadGamefromSlot "CheckpointSave"))
  (bind _output_get (Variables|/Game/Mechanics_Blockout/checpointSaveinfo.checpointSaveinfo_C|SetPlayer%20loc (.AsChecpoint%20Saveinfo (Utilities|Casting|CastTochecpointSaveinfo _returnvalue)) (Transformation|GetWorldLocation (Variables|Default|GetDefaultSceneRoot))))
  (SaveGame|SaveGametoSlot _returnvalue "CheckpointSave")
  (Development|PrintString (Utilities|String|ToString(Vector) _output_get))
  (Actor|DestroyActor))

(fn ConstructionScript)