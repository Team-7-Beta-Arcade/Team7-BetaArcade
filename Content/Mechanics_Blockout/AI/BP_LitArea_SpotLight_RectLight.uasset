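; Snatchable rect light with a lit zone that raises the player character's SightMod while they stand in its sphere.
; SnatchLight moves the light into or out of the player's capped held-light count, with a timeline-driven light actor flying between fixture and throw point.
; When the flight finishes, it swaps collision and shadow state between two linked shadow areas, resetting SightMod on switch-off if the old area is valid.
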(event OnComponentBeginOverlap(Sphere)
  (params (OverlappedComponent :type Primitive%20Component%20Object%20Reference) (OtherActor :type Actor%20Object%20Reference) (OtherComp :type Primitive%20Component%20Object%20Reference) (OtherBodyIndex :type Integer) (bFromSweep :type Boolean) (SweepResult :type Hit%20Result%20Structure%20%28by%20ref%29))
  (bind _returnvalue (Game|GetPlayerCharacter 0))
  (bind _asthird_person_character (Utilities|Casting|CastToThirdPersonCharacter _returnvalue))
  ;[1 1 1] Enter/Leave Lit area
  (if (Variables|Default|GetLightOn?)
    (if (== OtherActor _returnvalue)
      (Development|PrintString "PLAYER: LIT AREA" true true "(R=0.578125,G=0.000000,B=0.020287,A=1.000000)")
      (Variables|/Game/ThirdPersonBP/Blueprints/ThirdPersonCharacter.ThirdPersonCharacter_C|SetSightMod _asthird_person_character 5e+02)
      (Development|PrintString (Utilities|String|ToString(Float) (Variables|/Game/ThirdPersonBP/Blueprints/ThirdPersonCharacter.ThirdPersonCharacter_C|GetSightMod _asthird_person_character))))))

(event OnComponentEndOverlap(Sphere)
  (params (OverlappedComponent :type Primitive%20Component%20Object%20Reference) (OtherActor :type Actor%20Object%20Reference) (OtherComp :type Primitive%20Component%20Object%20Reference) (OtherBodyIndex :type Integer))
  (bind _returnvalue (Game|GetPlayerCharacter 0))
  (bind _asthird_person_character (Utilities|Casting|CastToThirdPersonCharacter _returnvalue))
  ;[1 1 1] Enter/Leave Lit area
  (if (Variables|Default|GetLightOn?)
    (if (== OtherActor (Game|GetPlayerCharacter 0))
      (Development|PrintString "PLAYER: LEFT LIT AREA" true true "(R=0.067629,G=1.000000,B=0.000000,A=1.000000)")
      (Variables|/Game/ThirdPersonBP/Blueprints/ThirdPersonCharacter.ThirdPersonCharacter_C|SetSightMod _asthird_person_character 0.0)
      (Development|PrintString (Utilities|String|ToString(Float) (Variables|/Game/ThirdPersonBP/Blueprints/ThirdPersonCharacter.ThirdPersonCharacter_C|GetSightMod _asthird_person_character))))))

(event Custom|LeftlitArea
  (bind _returnvalue (Game|GetPlayerCharacter 0))
  (bind _asthird_person_character (Utilities|Casting|CastToThirdPersonCharacter _returnvalue))
  ;[1 1 1] Enter/Leave Lit area
  (Variables|/Game/ThirdPersonBP/Blueprints/ThirdPersonCharacter.ThirdPersonCharacter_C|SetSightMod _asthird_person_character 0.0)
  (Development|PrintString (Utilities|String|ToString(Float) (Variables|/Game/ThirdPersonBP/Blueprints/ThirdPersonCharacter.ThirdPersonCharacter_C|GetSightMod _asthird_person_character))))

(event Custom|SnatchLight
  (params (Target :type Third%20Person%20Character%20Object%20Reference))
  ;[1 1 1] Snatch Light
  (Variables|Default|SetPlayer_REF Target)
  (if (Variables|Default|GetLightOn?)
    (Math|Integer|IncrementInt (Variables|/Game/ThirdPersonBP/Blueprints/ThirdPersonCharacter.ThirdPersonCharacter_C|GetCurrentlyHeldLights (Variables|Default|GetPlayer_REF))
      (:%20%20
        (if (> (Variables|/Game/ThirdPersonBP/Blueprints/ThirdPersonCharacter.ThirdPersonCharacter_C|GetCurrentlyHeldLights (Variables|Default|GetPlayer_REF)) 4)
          (Variables|/Game/ThirdPersonBP/Blueprints/ThirdPersonCharacter.ThirdPersonCharacter_C|SetCurrentlyHeldLights (Variables|Default|GetPlayer_REF) 4))
        (Variables|Default|SetLightOn? false)
        (Rendering|SetVisibility (Variables|Default|GetRectLight1) (Variables|Default|GetLightOn?) false)
        (bind _returnvalue (Game|SpawnActorfromClass "/Game/Mechanics_Blockout/BP_LightSnatch_Light.BP_LightSnatch_Light_C" (Math|Transform|MakeTransform (CallFunction|Location true) "0, 0, 0" "1,1,1") "AlwaysSpawn" 0 0 :!label _label))
        (Variables|Default|SetLight_REF _returnvalue)
        (bind (_direction _newtrack_0 _newtrack_1) (Timeline|Timeline_0 PlayFromStart)
          (:Update
            (Transformation|SetWorldLocation (Variables|/Script/Engine.Actor|GetRootComponent (Variables|Default|GetLight_REF)) (Math|Vector|Lerp(Vector) (CallFunction|Location true) (CallFunction|Location false) _newtrack_0) false false)
            (Transformation|SetActorScale3D (Variables|Default|GetLight_REF) (Math|Conversions|ToVector(Float) _newtrack_1)))
          (:Finished
            (Actor|DestroyActor (Variables|Default|GetLight_REF))
            (if (Variables|Default|GetLightOn?)
              (Rendering|SetVisibility (Variables|Default|GetRectLight1) (Variables|Default|GetLightOn?) false))
            (CallFunction|Activate/DeactivateShadowAreas)))))
    (elif (> (Variables|/Game/ThirdPersonBP/Blueprints/ThirdPersonCharacter.ThirdPersonCharacter_C|GetCurrentlyHeldLights (Variables|Default|GetPlayer_REF)) 0)
      (Math|Integer|DecrementInt (Variables|/Game/ThirdPersonBP/Blueprints/ThirdPersonCharacter.ThirdPersonCharacter_C|GetCurrentlyHeldLights (Variables|Default|GetPlayer_REF))
        (:%20%20
          (Variables|Default|SetLightOn? true)
          (goto _label))))))

(fn ConstructionScript
  (Rendering|SetVisibility (Variables|Default|GetRectLight1) (Variables|Default|GetLightOn?) false)
  (CallFunction|Activate/DeactivateShadowAreas))

(fn Activate/DeactivateShadowAreas
  (if (Variables|Default|GetLightOn?)
    ;[1 1 1] Turn light on
    (bind _shadowareanew (Variables|Default|GetShadowAreaNew)
      (:then
        (Collision|SetActorEnableCollision _shadowareanew true)
        (Default|ActivateShadow (Variables|/Game/Mechanics_Blockout/ShadowArea.ShadowArea_C|GetShadowComponenet _shadowareanew) true))
      (:else
        _))
    (bind _shadowareaold (Variables|Default|GetShadowAreaOld)
      (:then
        (Collision|SetActorEnableCollision _shadowareaold false)
        (Default|ActivateShadow (Variables|/Game/Mechanics_Blockout/ShadowArea.ShadowArea_C|GetShadowComponenet _shadowareaold) false))
      (:else))
    (else
      ;[1 1 1] Turn light off
      (bind _shadowareanew_2 (Variables|Default|GetShadowAreaNew)
        (:then
          (Collision|SetActorEnableCollision _shadowareanew_2 false)
          (Default|ActivateShadow (Variables|/Game/Mechanics_Blockout/ShadowArea.ShadowArea_C|GetShadowComponenet _shadowareanew_2) false))
        (:else
          _))
      (bind _shadowareaold_2 (Variables|Default|GetShadowAreaOld)
        (:then
          (Collision|SetActorEnableCollision _shadowareaold_2 true)
          (CallFunction|LeftlitArea)
          (Default|ActivateShadow (Variables|/Game/Mechanics_Blockout/ShadowArea.ShadowArea_C|GetShadowComponenet _shadowareaold_2) true))
        (:else)))))

(fn Location
  (params (Starting%20Loc? :type Boolean))
  (if Starting%20Loc?
    ;[1 1 1] Starting location
    (if (not (Variables|Default|GetLightOn?))
      (return (Transformation|GetWorldLocation (Variables|Default|GetStaticMesh)))
      (else
        (return (Transformation|GetWorldLocation (Variables|/Game/ThirdPersonBP/Blueprints/ThirdPersonCharacter.ThirdPersonCharacter_C|GetThrow_ItemLOC (Variables|Default|GetPlayer_REF))))))
    (else
      ;[1 1 1] End Location
      (if (not (Variables|Default|GetLightOn?))
        (return (Transformation|GetWorldLocation (Variables|/Game/ThirdPersonBP/Blueprints/ThirdPersonCharacter.ThirdPersonCharacter_C|GetThrow_ItemLOC (Variables|Default|GetPlayer_REF))))
        (else
          (return (Transformation|GetWorldLocation (Variables|Default|GetStaticMesh))))))))