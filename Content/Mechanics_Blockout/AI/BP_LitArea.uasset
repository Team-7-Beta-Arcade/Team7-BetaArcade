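; BP_LitArea is a switchable light zone that raises the player character's SightMod while inside it, likely affecting AI detection.
; Sphere overlaps set or clear the modifier only while the light is on, printing debug messages.
; TurnOnOffLight toggles the spotlight and swaps collision and shadow activation between ShadowAreaNew and ShadowAreaOld.
; Switching off also resets SightMod, but only when ShadowAreaOld is valid.
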(event OnComponentBeginOverlap(Sphere)
  (params (OverlappedComponent :type Primitive%20Component%20Object%20Reference) (OtherActor :type Actor%20Object%20Reference) (OtherComp :type Primitive%20Component%20Object%20Reference) (OtherBodyIndex :type Integer) (bFromSweep :type Boolean) (SweepResult :type Hit%20Result%20Structure%20%28by%20ref%29))
  (bind _returnvalue (Game|GetPlayerCharacter 0))
  (bind _asthird_person_character (Utilities|Casting|CastToThirdPersonCharacter _returnvalue))
  ;[1 1 1] Enter/Leave Lit area
  (if (Variables|Default|GetLightOn?)
    (if (== OtherActor _returnvalue)
      (Development|PrintString "PLAYER: LIT AREA" true true "(R=0.578125,G=0.000000,B=0.020287,A=1.000000)")
      (Variables|/Game/ThirdPersonBP/Blueprints/ThirdPersonCharacter.ThirdPersonCharacter_C|SetSightMod _asthird_person_character 5e+02)
      (Development|PrintString (Utilities|String|ToString(Float) (Variables|/Game/ThirdPersonBP/Blueprints/ThirdPersonCharacter.ThirdPersonCharacter_C|GetSightMod _asthird_person_character))))))

(event OnComponentEndOverlap(Sphere)
  (params (OverlappedComponent :type Primitive%20Component%20Object%20Reference) (OtherActor :type Actor%20Object%20Reference) (OtherComp :type Primitive%20Component%20Object%20Reference) (OtherBodyIndex :type Integer))
  (bind _returnvalue (Game|GetPlayerCharacter 0))
  (bind _asthird_person_character (Utilities|Casting|CastToThirdPersonCharacter _returnvalue))
  ;[1 1 1] Enter/Leave Lit area
  (if (Variables|Default|GetLightOn?)
    (if (== OtherActor (Game|GetPlayerCharacter 0))
      (Development|PrintString "PLAYER: LEFT LIT AREA" true true "(R=0.067629,G=1.000000,B=0.000000,A=1.000000)")
      (Variables|/Game/ThirdPersonBP/Blueprints/ThirdPersonCharacter.ThirdPersonCharacter_C|SetSightMod _asthird_person_character 0.0)
      (Development|PrintString (Utilities|String|ToString(Float) (Variables|/Game/ThirdPersonBP/Blueprints/ThirdPersonCharacter.ThirdPersonCharacter_C|GetSightMod _asthird_person_character))))))

(event Custom|LeftlitArea
  (bind _returnvalue (Game|GetPlayerCharacter 0))
  (bind _asthird_person_character (Utilities|Casting|CastToThirdPersonCharacter _returnvalue))
  ;[1 1 1] Enter/Leave Lit area
  (Variables|/Game/ThirdPersonBP/Blueprints/ThirdPersonCharacter.ThirdPersonCharacter_C|SetSightMod _asthird_person_character 0.0)
  (Development|PrintString (Utilities|String|ToString(Float) (Variables|/Game/ThirdPersonBP/Blueprints/ThirdPersonCharacter.ThirdPersonCharacter_C|GetSightMod _asthird_person_character))))

(fn ConstructionScript)

(fn TurnOn/OffLight
  (params (bNewActive :type Boolean))
  (Variables|Default|SetLightOn? bNewActive)
  (Rendering|SetVisibility (Variables|Default|GetSpotLight) bNewActive false)
  (if bNewActive
    ;[1 1 1] Turn light on
    (bind _shadowareanew (Variables|Default|GetShadowAreaNew)
      (:then
        (Collision|SetActorEnableCollision _shadowareanew true)
        (Default|ActivateShadow (Variables|/Game/Mechanics_Blockout/ShadowArea.ShadowArea_C|GetShadowComponenet _shadowareanew) true))
      (:else
        _))
    (bind _shadowareaold (Variables|Default|GetShadowAreaOld)
      (:then
        (Collision|SetActorEnableCollision _shadowareaold false)
        (Default|ActivateShadow (Variables|/Game/Mechanics_Blockout/ShadowArea.ShadowArea_C|GetShadowComponenet _shadowareaold) false))
      (:else))
    (else
      ;[1 1 1] Turn light off
      (bind _shadowareanew_2 (Variables|Default|GetShadowAreaNew)
        (:then
          (Collision|SetActorEnableCollision _shadowareanew_2 false)
          (Default|ActivateShadow (Variables|/Game/Mechanics_Blockout/ShadowArea.ShadowArea_C|GetShadowComponenet _shadowareanew_2) false))
        (:else
          _))
      (bind _shadowareaold_2 (Variables|Default|GetShadowAreaOld)
        (:then
          (Collision|SetActorEnableCollision _shadowareaold_2 true)
          (CallFunction|LeftlitArea)
          (Default|ActivateShadow (Variables|/Game/Mechanics_Blockout/ShadowArea.ShadowArea_C|GetShadowComponenet _shadowareaold_2) true))
        (:else)))))