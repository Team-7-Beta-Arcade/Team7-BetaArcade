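; BP_ShadowComponenet is a component for BP_ShadowArea that switches a shadow on and off, starting on when StartsActive is set.
; Activation traces downward from the component, spawns an ActorShadowTest at the impact point as ShadowPoint, attaches it to the owner and shows PShadowArea.
; ActivateShadow repeats this when its condition is true, otherwise it hides PShadowArea and destroys ShadowPoint.
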(event Custom|ActivateShadow
  (params (Condition :type Boolean))
  (bind _returnvalue (Transformation|GetWorldLocation))
  (bind (_x _y _z) (Math|Vector|BreakVector _returnvalue))
  (if Condition
    (bind _outhit (Collision|LineTraceByChannel (Transformation|GetWorldLocation) (Math|Vector|MakeVector _x _y (- _z 5e+02)) "TraceTypeQuery1" false 0 "None"))
    (bind _returnvalue_2 (Game|SpawnActorfromClass "/Game/Mechanics_Blockout/ActorShadowTest.ActorShadowTest_C" (Math|Transform|MakeTransform (.ImpactPoint (Collision|BreakHitResult _outhit)) "0, 0, 0" "1,1,1") "AlwaysSpawn" 0 0))
    (bind _output_get (Variables|Default|SetShadowPoint _returnvalue_2))
    (Transformation|AttachActorToActor _returnvalue_2 (Components|GetOwner) "None" "KeepWorld" "KeepWorld" "KeepWorld" true)
    (Rendering|SetVisibility (Variables|/Game/Mechanics_Blockout/BP_ShadowArea.BP_ShadowArea_C|GetP_ShadowArea (.AsShadow%20Area (Utilities|Casting|CastToBP_ShadowArea (Components|GetOwner)))) true false)
    (else
      (Rendering|SetVisibility (Variables|/Game/Mechanics_Blockout/BP_ShadowArea.BP_ShadowArea_C|GetP_ShadowArea (.AsShadow%20Area (Utilities|Casting|CastToBP_ShadowArea (Components|GetOwner)))) false false)
      (bind _shadowpoint (Variables|Default|GetShadowPoint)
        (:then
          (Actor|DestroyActor _shadowpoint))
        (:else)))))

(event EventBeginPlay
  (bind _returnvalue (Transformation|GetWorldLocation))
  (bind (_x _y _z) (Math|Vector|BreakVector _returnvalue))
  (if (Variables|Default|GetStartsActive?)
    (bind _outhit (Collision|LineTraceByChannel (Transformation|GetWorldLocation) (Math|Vector|MakeVector _x _y (- _z 5e+02)) "TraceTypeQuery1" false 0 "None"))
    (bind _returnvalue_2 (Game|SpawnActorfromClass "/Game/Mechanics_Blockout/ActorShadowTest.ActorShadowTest_C" (Math|Transform|MakeTransform (.ImpactPoint (Collision|BreakHitResult _outhit)) "0, 0, 0" "1,1,1") "AlwaysSpawn" 0 0))
    (bind _output_get (Variables|Default|SetShadowPoint _returnvalue_2))
    (Transformation|AttachActorToActor _returnvalue_2 (Components|GetOwner) "None" "KeepWorld" "KeepWorld" "KeepWorld" true)
    (Rendering|SetVisibility (Variables|/Game/Mechanics_Blockout/BP_ShadowArea.BP_ShadowArea_C|GetP_ShadowArea (.AsShadow%20Area (Utilities|Casting|CastToBP_ShadowArea (Components|GetOwner)))) true false)))