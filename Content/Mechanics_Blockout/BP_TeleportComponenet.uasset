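; Player controller component that picks the shadow actor the player can teleport to; it does not perform the teleport.
; CheckOwner caches the controlled pawn (player, enemy or possession camera) to supply search origin and view direction.
; LookForTP starts a looping timer that sphere-overlaps shadows, line-traces for visibility and favors the smallest camera angle within a cone.
; SetNewTarget toggles target active state; searching pauses during teleports, and AttemptTeleport is a stub.
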(event Custom|CheckOwner
  (bind _returnvalue (Components|GetOwner))
  (bind _asplayer_con (Utilities|Casting|CastToBP_PlayerCon _returnvalue))
  (bind _returnvalue_2 (Pawn|GetControlledPawn _asplayer_con))
  ;[1 1 1] Check if player is possessing Player pawn or Enemy pawn
  (bind _asthird_person_character (Utilities|Casting|CastToThirdPersonCharacter _returnvalue_2)
    (:then
      (Variables|Default|SetOwnedByPlayer? true)
      (Variables|Default|SetOwningCharacter _asthird_person_character))
    (:CastFailed
      (bind _asenemy (Utilities|Casting|CastToEnemy _returnvalue_2)
        (:then
          (Variables|Default|SetOwnedByPlayer? false)
          (Variables|Default|SetEnemyOwningCharacter _asenemy))
        (:CastFailed
          (bind _ascamera_pawn (Utilities|Casting|CastToBP_CameraPawn_Possession _returnvalue_2))
          (Variables|Default|SetOwnedByPlayer? false)
          (Variables|Default|SetOwningCameraPawn _ascamera_pawn))))))

(event Custom|LookForTP
  ;[1 1 1] Search for teleport location
  (Utilities|Time|SetTimerbyFunctionName 0 "FindBestTeleportLocation" 0.05 true))

(event EventBeginPlay
  (bind _returnvalue (Components|GetOwner))
  (bind _asplayer_con (Utilities|Casting|CastToBP_PlayerCon _returnvalue))
  (bind _returnvalue_2 (Pawn|GetControlledPawn _asplayer_con))
  ;[1 1 1] Check if player is possessing Player pawn or Enemy pawn
  (Variables|Default|SetPlayerController_REF _asplayer_con)
  (bind _asthird_person_character (Utilities|Casting|CastToThirdPersonCharacter _returnvalue_2)
    (:then
      (Variables|Default|SetOwnedByPlayer? true)
      (Variables|Default|SetOwningCharacter _asthird_person_character))
    (:CastFailed
      (bind _asenemy (Utilities|Casting|CastToEnemy _returnvalue_2)
        (:then
          (Variables|Default|SetOwnedByPlayer? false)
          (Variables|Default|SetEnemyOwningCharacter _asenemy))
        (:CastFailed
          (bind _ascamera_pawn (Utilities|Casting|CastToBP_CameraPawn_Possession _returnvalue_2))
          (Variables|Default|SetOwnedByPlayer? false)
          (Variables|Default|SetOwningCameraPawn _ascamera_pawn))))))

(fn FindBestTarget
  (params (Targets :type Array%20of%20Actor%20Object%20References))
  (for _array_element Targets
    (LocalVariables|SetCurrentTarget%28Local%29 _array_element)
    (bind (_outhit _returnvalue) (Collision|LineTraceByChannel (CallFunction|OwnerLocation) (Transformation|GetActorLocation (LocalVariables|GetCurrentTarget%28Local%29)) "TraceTypeQuery3" false (Utilities|Array|MakeArray (Variables|Default|GetOwningCharacter) (Variables|Default|GetEnemyOwningCharacter) (CallFunction|CheckifValid)) "ForDuration" true "(R=1.000000,G=0.000000,B=0.000000,A=1.000000)" "(R=0.000000,G=1.000000,B=0.000000,A=1.000000)" 0.5))
    (if _returnvalue
      (if (== (.HitActor (Collision|BreakHitResult _outhit)) (LocalVariables|GetCurrentTarget%28Local%29))
        (Utilities|FlowControl|Sequence
          (:then_0
            (LocalVariables|SetCurrentAngle%28Local%29 (Class|KismetMathLibrary|DegAcos (Math|Vector|DotProduct (Math|Vector|Normalize (- (Transformation|GetActorLocation (LocalVariables|GetCurrentTarget%28Local%29)) (CallFunction|OwnerLocation))) (CallFunction|OwnerCamera)))))
          (:then_1
            (if (or (< (LocalVariables|GetCurrentAngle%28Local%29) (LocalVariables|GetBestAngle%28Local%29)) (not (Utilities|IsValid (LocalVariables|GetBestTarget%28Local%29))))
              (LocalVariables|SetBestTarget%28Local%29 (LocalVariables|GetCurrentTarget%28Local%29))
              (LocalVariables|SetBestAngle%28Local%29 (LocalVariables|GetCurrentAngle%28Local%29))))
          (:then_2
            (if (> (LocalVariables|GetBestAngle%28Local%29) 3e+01)
              (LocalVariables|SetBestTarget%28Local%29 0)
              (LocalVariables|SetBestAngle%28Local%29 0.0)))))))
  (return (LocalVariables|GetBestTarget%28Local%29)))

(fn SetNewTarget
  (params (NewTarget :type Actor%20Shadow%20Test%20Object%20Reference))
  (if (!= NewTarget (Variables|Default|GetCurrentTarget))
    (Utilities|FlowControl|Sequence
      (:then_0
        (bind _currenttarget (Variables|Default|GetCurrentTarget)
          (:then
            (Default|SetActive _currenttarget false))
          (:else)))
      (:then_1
        (Variables|Default|SetCurrentTarget NewTarget))
      (:then_2
        (bind _currenttarget_2 (Variables|Default|GetCurrentTarget)
          (:then
            (Default|SetActive _currenttarget_2 true))
          (:else))))))

(fn AttemptTeleport
  (if (Variables|/Game/ThirdPersonBP/Blueprints/ThirdPersonCharacter.ThirdPersonCharacter_C|GetCanBeSeen? (Variables|Default|GetOwningCharacter))
    _))

(fn OwnerLocation
  (Variables|Default|GetEnemyOwningCharacter
    (:then
      (return (CallFunction|ChooseValidOwnerLocation (Variables|Default|GetEnemyOwningCharacter))))
    (:else
      (Variables|Default|GetOwningCameraPawn
        (:then
          (return (CallFunction|ChooseValidOwnerLocation (Actor|GetAttachParentActor (Variables|Default|GetOwningCameraPawn)))))
        (:else
          (return (CallFunction|ChooseValidOwnerLocation)))))))

(fn FindBestTeleportLocation
  (if (Variables|/Game/Mechanics_Blockout/BP_PlayerCon.BP_PlayerCon_C|GetIsTeleporting? (Variables|Default|GetPlayerController_REF))
    (Class|KismetSystemLibrary|PauseTimer 0 "FindBestTeleportLocation")
    (else
      (bind _outactors (Collision|SphereOverlapActors (CallFunction|OwnerLocation) (Variables|Default|GetMaxTeleportDistance) (Utilities|Array|MakeArray "ObjectTypeQuery1") "/Game/Mechanics_Blockout/ActorShadowTest.ActorShadowTest_C" (Utilities|Array|MakeArray (Variables|/Game/Mechanics_Blockout/BP_PlayerCon.BP_PlayerCon_C|GetCurrentOccupiedShadow (Variables|Default|GetPlayerController_REF)))))
      (bind _closesttarget (CallFunction|FindBestTarget _outactors))
      (bind _asactor_shadow_test (Utilities|Casting|CastToActorShadowTest _closesttarget)
        (:then
          (CallFunction|SetNewTarget _asactor_shadow_test))
        (:CastFailed
          (CallFunction|SetNewTarget))))))

(fn ResetCurrentTarget
  (Class|KismetSystemLibrary|PauseTimer 0 "FindBestTeleportLocation")
  (bind _currenttarget (Variables|Default|GetCurrentTarget)
    (:then
      (Default|SetActive _currenttarget false)
      (Variables|Default|SetCurrentTarget 0)
      (return))
    (:else)))

(fn OwnerCamera
  (Variables|Default|GetEnemyOwningCharacter
    (:then
      (return (CallFunction|ChooseValidOwnerCamera (Variables|/Game/Mechanics_Blockout/AI/Enemy.Enemy_C|GetCamera (Variables|Default|GetEnemyOwningCharacter)))))
    (:else
      (Variables|Default|GetOwningCameraPawn
        (:then
          (return (CallFunction|ChooseValidOwnerCamera (Variables|/Game/Mechanics_Blockout/BP_CameraPawn_Possession.BP_CameraPawn_Possession_C|GetCamera (Variables|Default|GetOwningCameraPawn)))))
        (:else
          (return (CallFunction|ChooseValidOwnerCamera)))))))

(fn CheckifValid
  (bind _owningcamerapawn (Variables|Default|GetOwningCameraPawn)
    (:then
      (return (Actor|GetAttachParentActor _owningcamerapawn)))
    (:else)))

(fn ChooseValidOwnerLocation
  (params (Target :type Actor%20Object%20Reference))
  (bind _owningcharacter (Variables|Default|GetOwningCharacter))
  (bind _returnvalue (Transformation|GetActorLocation _owningcharacter))
  (if (Utilities|IsValid Target)
    (return (select (Variables|Default|GetOwnedByPlayer?) _returnvalue (Transformation|GetActorLocation Target)))
    (else
      (return _returnvalue))))

(fn ChooseValidOwnerCamera
  (params (Target :type Scene%20Component%20Object%20Reference))
  (bind _owningcharacter (Variables|Default|GetOwningCharacter))
  (bind _followcamera (Variables|/Game/ThirdPersonBP/Blueprints/ThirdPersonCharacter.ThirdPersonCharacter_C|GetFollowCamera _owningcharacter))
  (bind _returnvalue (Math|Vector|GetForwardVector _followcamera))
  (if (Utilities|IsValid Target)
    (return (select (Variables|Default|GetOwnedByPlayer?) _returnvalue (Math|Vector|GetForwardVector Target)))
    (else
      (return _returnvalue))))